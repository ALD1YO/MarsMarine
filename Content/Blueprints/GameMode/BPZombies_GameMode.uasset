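; Game mode that runs escalating waves of zombies, starting shortly after play begins.
; Each wave multiplies the difficulty to set its spawn count, then a looping timer spawns zombies at random TargetPoint actors until that count runs out.
; Living zombies are tracked in an array; when a registered death leaves it empty with no spawns remaining, the next wave starts after a short delay.
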(event Custom|Spawn%20Wave
  (CallFunction|SpawnZombie))

(event Custom|End%20Wave
  (Utilities|FlowControl|Delay 2.0)
  (CallFunction|StartNewWave))

(event EventBeginPlay
  (Utilities|FlowControl|Delay 2.0)
  (CallFunction|StartNewWave))

(fn ConstructionScript)

(fn StartNewWave
  (Math|Integer|IncrementInt (Variables|Default|GetCurrent%20Wave)
    (:%20%20
      (CallFunction|IncreaseWaveDifficulty)
      (Utilities|Time|SetTimerbyFunctionName 0 "Spawn Wave" (Variables|Default|GetSpawn%20Frecuency) true))))

(fn SpawnZombie
  (bind _spawn_point (CallFunction|GetRandomSpawnPoint))
  (Utilities|IsValid _spawn_point
    (:Is%20Valid
      (bind _returnvalue (Game|SpawnActorfromClass "/Game/Blueprints/AI/BP_Zombie.BP_Zombie_C" (Transformation|GetActorTransform _spawn_point) "Undefined" 0 0))
      (Utilities|IsValid _returnvalue
        (:Is%20Valid
          (Utilities|Array|Add (Variables|Default|GetZombies) _returnvalue)
          (bind _result (Math|Integer|DecrementInt (Variables|Default|GetZombies%20Spawns%20Remaining))
            (:%20%20
              (if (== _result 0)
                (Utilities|Time|ClearTimerbyFunctionName 0 "Spawn Wave")))))))))

(fn GetRandomSpawnPoint
  (bind _outactors (Actor|GetAllActorsOfClass "/Script/Engine.TargetPoint"))
  (return (Utilities|Array|Get(acopy) _outactors (Math|Random|RandomIntegerinRange 0 (Utilities|Array|LastIndex _outactors)))))

(fn IsWaveComplete
  (return (and (== (Utilities|Array|Length (Variables|Default|GetZombies)) 0) (== (Variables|Default|GetZombies%20Spawns%20Remaining) 0))))

(fn IncreaseWaveDifficulty
  (bind _output_get (Variables|Default|SetWave%20Difficulty (Math|Float|Round (* (Variables|Default|GetWave%20Difficulty) (Variables|Default|GetDificulty%20Multiplier)))))
  (Variables|Default|SetZombies%20Spawns%20Remaining _output_get))

(fn RegisterZombieDeath
  (params (Zombie :type BP%20Zombie%20Object%20Reference%20%28by%20ref%29))
  (Utilities|Array|RemoveItem (Variables|Default|GetZombies) Zombie)
  (if (CallFunction|IsWaveComplete)
    (CallFunction|EndWave)))